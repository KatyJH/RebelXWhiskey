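; BP_Level_Checkpoint is a trigger box that acts as a level checkpoint for Player_RebelX, with its size set in the Construction Script.
; When active and overlapped by the player, it runs optional steps, each gated by a flag.
; It saves the player's current transform as the respawn point with a HUD notification, updates the HUD objective once, or destroys itself after a short delay.
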(event OnComponentBeginOverlap(Box)
  (params (OverlappedComponent :type Primitive%20Component%20Object%20Reference) (OtherActor :type Actor%20Object%20Reference) (OtherComp :type Primitive%20Component%20Object%20Reference) (OtherBodyIndex :type Integer) (bFromSweep :type Boolean) (SweepResult :type Hit%20Result%20Structure%20%28by%20ref%29))
  (bind _asplayer_rebel_x (Utilities|Casting|CastToPlayer_RebelX OtherActor))
  (Variables|Default|SetAs%20Player%20Rebel%20X _asplayer_rebel_x)
  (if (Variables|RebelX|GetActive?)
    (Utilities|FlowControl|Sequence
      (:then_0
        ;[0.15 0.15 0.15 0.5] Set Respawn Point
        (if (Variables|RebelX|Checkpoint|GetRespawn%20Checkpoint?)
          (Variables|/Game/RebelX_Core/Blueprints/Player_RebelX.Player_RebelX_C|SetRespawn%20Transform (Variables|Default|GetAs%20Player%20Rebel%20X) (Transformation|GetActorTransform (Variables|Default|GetAs%20Player%20Rebel%20X)))
          (Class|BPIHUD|AddNotificaiton(Message) (Default|GetAttachedHUD (Variables|Default|GetAs%20Player%20Rebel%20X)) (Variables|RebelX|Checkpoint|GetNotification%20Text))))
      (:then_1
        ;[0.15 0.15 0.15 0.5] Update Objective
        (if (Variables|RebelX|ObjectiveUpdate|GetUpdate%20Objective?)
          (Utilities|FlowControl|DoOnce false
            (:Completed
              (Class|BPIHUD|UpdateObjective(Message) (HUD|GetHUD (Game|GetPlayerController 0)) (Variables|RebelX|ObjectiveUpdate|GetObjective%20Title) (Variables|RebelX|ObjectiveUpdate|GetObjective%20Details))))))
      (:then_2
        ;[0.15 0.15 0.15 0.5] Destroy after use
        (if (Variables|RebelX|GetDestory%20after%20use?)
          (Utilities|FlowControl|Delay 0.2)
          (Actor|DestroyActor))))))

(event EventBeginPlay)

(event Collision|EventActorBeginOverlap
  (params (OtherActor :type Actor%20Object%20Reference)))

(event EventTick
  (params (DeltaSeconds :type Float%20%28single-precision%29)))

(fn ConstructionScript
  (Components|Box|SetBoxExtent (Variables|Default|GetBox) (Variables|RebelX|Checkpoint|GetBox%20Extent) true))